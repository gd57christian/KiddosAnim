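; BP_fallingRock is a rock actor that travels along a spline on BeginPlay, then triggers a linked jump gem.
; It takes the BP_spline found in the level and uses the MoveObject timeline to drive its location and rotation along the full length.
; Collision stays off during the move, then turns on before GemJump is called.
; The construction script applies exposed mass and damping values and derives the timeline play rate from a completion time.
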(event Custom|FallRockStart
  (bind _splineref (Variables|Default|GetsplineRef))
  (bind _spline (Variables|/Game/Blueprint/BP_spline.BP_spline_C|GetSpline _splineref))
  (bind _movementtime (Timeline|MoveObject Play)
    (:Update
      (Transformation|SetActorTransform (Math|Transform|MakeTransform (Spline|GetLocationatDistanceAlongSpline _spline (Math|Float|Lerp 0.0 (Spline|GetSplineLength (Variables|/Game/Blueprint/BP_spline.BP_spline_C|GetSpline _splineref)) _movementtime) "World") (Spline|GetRotationatDistanceAlongSpline _spline (Math|Float|Lerp 0.0 (Spline|GetSplineLength (Variables|/Game/Blueprint/BP_spline.BP_spline_C|GetSpline _splineref)) _movementtime) "World") "1,1,1")))
    (:Finished
      (Collision|SetCollisionEnabled (Variables|Default|GetBig_Rock_LP_DM) "QueryAndPhysics")
      (bind _asbp_jump_gem_2 (Utilities|Casting|CastToBP_jumpGem2 (Variables|Default|GetJumpGem2)))
      (Default|GemJump _asbp_jump_gem_2))))

(event EventBeginPlay
  ;[1 1 1] Begin Play setting spline and start fall the rock
  (bind _returnvalue (Actor|GetActorOfClass "/Game/Blueprint/BP_spline.BP_spline_C"))
  (Variables|Default|SetsplineRef _returnvalue)
  (Collision|SetCollisionEnabled (Variables|Default|GetBig_Rock_LP_DM) "NoCollision")
  (CallFunction|FallRockStart))

(fn ConstructionScript
  (bind _big_rock_lp_dm (Variables|Default|GetBig_Rock_LP_DM))
  ;[1 1 1] Exposing Variables
  (Class|PrimitiveComponent|SetMassScale _big_rock_lp_dm "None" (Variables|Default|GetIn%20Mass%20Scale))
  (Class|PrimitiveComponent|SetAngularDamping _big_rock_lp_dm (Variables|Default|GetAngularDampling))
  (Class|PrimitiveComponent|SetLinearDamping _big_rock_lp_dm (Variables|Default|GetLinear%20Damping))
  ;[1 1 1] Setting Play rate of the timeline in seconds
  (Components|Timeline|SetPlayRate (Variables|Default|GetMoveObject) (/ 1.0 (Variables|Default|GetTImetoComplete_seconds))))