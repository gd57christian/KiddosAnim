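; BP_CrumblingRock is a rock that breaks apart through its Destructible component as soon as play begins.
; BeginPlay applies damage at the component's location, with a configurable impulse along its up vector.
; A Crumble timeline for shaking and swaying before the break is present but never triggered, as are a pause delay and play-rate calls.
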(event EventBeginPlay
  (bind _destructible (Variables|Default|GetDestructible))
  (Class|DestructibleComponent|ApplyDamage _destructible 1e+02 (Transformation|GetWorldLocation _destructible) (Math|Vector|GetUpVector _destructible) (Variables|Variables|GetExplodeImpulseStreng)))

(event Collision|EventActorBeginOverlap
  (params (OtherActor :type Actor%20Object%20Reference)))

(event EventTick
  (params (DeltaSeconds :type Float%20%28single-precision%29)))

(fn ConstructionScript)