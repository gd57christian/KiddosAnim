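; BP_JumpGem is an actor that travels along its own spline path when its JumpGem event is called.
; The MoveObject timeline drives a lerp over the spline's length, moving the actor to that world-space location each update; spline rotation is left unused.
; The construction script sets the timeline play rate to the inverse of TImetoCompleteSeconds to control travel time.
; BeginPlay is empty, so movement waits for that event.
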(event Custom|JumpGem
  (bind _spline (Variables|Default|GetSpline))
  (bind _movementtime (Timeline|MoveObject Play)
    (:Update
      (Transformation|SetActorTransform (Math|Transform|MakeTransform (Spline|GetLocationatDistanceAlongSpline _spline (Math|Float|Lerp 0.0 (Spline|GetSplineLength _spline) _movementtime) "World") "0, 0, 0" "1,1,1")))))

(event EventBeginPlay
  ;[1 1 1] Begin Play setting spline and start fall the rock
)

(fn ConstructionScript
  ;[1 1 1] Setting Play rate of the timeline in seconds
  (Components|Timeline|SetPlayRate (Variables|Default|GetMoveObject) (/ 1.0 (Variables|VariableRock|GetTImetoComplete_seconds))))