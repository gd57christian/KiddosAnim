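; Gem actor that, when its GemJump event fires, becomes visible and travels along a spline path.
; At BeginPlay it caches a BP_spline2 actor found in the level.
; The GemMov timeline drives a lerp over the spline's length, moving the actor to that world location each update.
; The construction script sets the timeline play rate from Timetocomplete, so that variable controls the travel duration.
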(event Custom|GemJump
  (bind _gemspline (Variables|Default|Getgemspline))
  (bind _spline (Variables|/Game/Blueprint/BP_spline2.BP_spline2_C|GetSpline _gemspline))
  (Rendering|SetVisibility (Variables|Default|GetGem) true false)
  (bind _newtrack_0 (Timeline|GemMov Play)
    (:Update
      (Transformation|SetActorLocation (Spline|GetLocationatDistanceAlongSpline _spline (Math|Float|Lerp 0.0 (Spline|GetSplineLength _spline) _newtrack_0) "World") false false))))

(event EventBeginPlay
  (bind _returnvalue (Actor|GetActorOfClass "/Game/Blueprint/BP_spline2.BP_spline2_C"))
  (Variables|Default|Setgemspline _returnvalue))

(fn ConstructionScript
  (Components|Timeline|SetPlayRate (Variables|Default|GetGemMov) (/ 1.0 (Variables|Default|Gettimetocomplete))))